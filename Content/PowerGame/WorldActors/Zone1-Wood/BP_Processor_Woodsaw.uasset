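; BP_Processor_Woodsaw is a wood-zone processor actor that adds a spinning saw animation to its parent class.
; On BeginPlay it calls the parent, then plays the SawRotation timeline, whose Alpha lerps Arrow0's relative rotation through a full 360-degree turn on one axis.
; It adds no other logic: the construction script only calls the parent, and Tick and overlap events are disabled.
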(event EventBeginPlay
  (|CallParentFunction)
  (bind _alpha (Timeline|SawRotation Play)
    (:Update
      (Transformation|SetRelativeRotation (Variables|Default|GetArrow_0) (Math|Rotator|Lerp(Rotator) "0.000000,90.000000,0.000000" "0.000000,90.000000,360.000000" _alpha) false false))))

(event Collision|EventActorBeginOverlap
  (params (OtherActor :type Actor%20Object%20Reference))
  (|CallParentFunction OtherActor) ; This node is disabled and will not be called.\nDrag off pins to build functionality.
)

(event EventTick
  (params (DeltaSeconds :type Float%20%28single-precision%29))
  (|CallParentFunction DeltaSeconds) ; This node is disabled and will not be called.\nDrag off pins to build functionality.
)

(fn ConstructionScript
  (|CallParentFunction))