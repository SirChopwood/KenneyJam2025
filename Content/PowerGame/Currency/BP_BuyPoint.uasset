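; BP_BuyPoint is a purchase pad that, when the player overlaps it with enough currency and no pending prerequisites, charges the cost and destroys itself.
; At BeginPlay it records and removes non-upgradeable placed actors, and hides itself while prerequisite buy points remain.
; Purchase either unlocks a zone or respawns stored actors and swaps others via the ActorUpgrades class map.
; OnPurchased passes spawned actors to dependent points for later upgrades.
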(event OnComponentBeginOverlap(Box)
  (params (OverlappedComponent :type Primitive%20Component%20Object%20Reference) (OtherActor :type Actor%20Object%20Reference) (OtherComp :type Primitive%20Component%20Object%20Reference) (OtherBodyIndex :type Integer) (bFromSweep :type Boolean) (SweepResult :type Hit%20Result%20Structure%20%28by%20ref%29))
  (if (== (Game|Player|GetPlayerPawn 0) OtherActor)
    (if (and (Utilities|Array|IsEmpty (Variables|Runtime|GetPreRequesites)) (>= (Variables|/Game/PowerGame/Core/BP_PowerGameMode.BP_PowerGameMode_C|GetCurrency (Variables|Runtime|GetGameMode)) (Variables|/Game/PowerGame/Currency/PDA_Purchase.PDA_Purchase_C|GetCost (Variables|Setup|GetPurchase))))
      (Utilities|FlowControl|DoOnce false
        (:Completed
          (CallFunction|CompletePurchase)
          (Utilities|FlowControl|DelayUntilNextTick)
          (Actor|DestroyActor))))))

(event Custom|OnPrerequesitePurchased
  (params (PurchasedBuyPoint :type BP%20Buy%20Point%20Object%20Reference) (PurchasedActors :type Array%20of%20Actor%20Object%20References))
  (bind _prerequesites (Variables|Runtime|GetPreRequesites))
  (Utilities|Array|RemoveItem _prerequesites PurchasedBuyPoint)
  (Rendering|SetActorHiddenInGame (Utilities|Array|IsNotEmpty _prerequesites))
  (bind _keys (Utilities|Map|Keys (Variables|Setup|GetActorUpgrades)))
  (for _array_element PurchasedActors
    (if (Utilities|Array|ContainsItem _keys (Utilities|GetClass _array_element))
      (Utilities|Array|Add (Variables|Setup|GetActorAdditions) _array_element))))

(event EventBeginPlay
  (bind _asbp_power_game_mode (Utilities|Casting|CastToBP_PowerGameMode (Game|GetGameMode)))
  (Variables|Runtime|SetGameMode _asbp_power_game_mode)
  (Utilities|FlowControl|DelayUntilNextTick)
  (CallFunction|InitSpawnableActors (Variables|Setup|GetActorAdditions))
  (Utilities|FlowControl|DelayUntilNextTick)
  (CallFunction|InitPrerequesites))

(fn ConstructionScript)

(fn InitSpawnableActors
  (params (Actor%20Array :type Array%20of%20Actor%20Object%20References))
  (bind _keys (Utilities|Map|Keys (Variables|Setup|GetActorUpgrades)))
  (for _array_element Actor%20Array
    (if (not (Utilities|Array|ContainsItem _keys (Utilities|GetClass _array_element)))
      (Utilities|Array|Add (Variables|Runtime|GetTargetTransforms) (Transformation|GetActorTransform _array_element))
      (Utilities|Array|Add (Variables|Runtime|GetTargetClasses) (Utilities|GetClass _array_element))
      (Actor|DestroyActor _array_element)))
  (return))

(fn InitPrerequesites
  (bind _outactors (Actor|GetAllActorsOfClass "BP_BuyPoint_C"))
  (for _array_element _outactors
    (if (Utilities|Array|ContainsItem (Variables|/Game/PowerGame/Currency/PDA_Purchase.PDA_Purchase_C|GetPreRequesites (Variables|Setup|GetPurchase)) (Variables|BP_BuyPoint_C|GetPurchase _array_element))
      (Utilities|Array|Add (Variables|Runtime|GetPreRequesites) _array_element)
      (EventDispatchers|BindEventtoOnPurchased _array_element (EventDispatchers|CreateEvent :!event Custom|OnPrerequesitePurchased))))
  (Rendering|SetActorHiddenInGame (Utilities|Array|IsNotEmpty (Variables|Runtime|GetPreRequesites))))

(fn CompletePurchase
  (bind _levelunlock (Variables|Setup|GetLevelUnlock))
  (Utilities|FlowControl|Sequence
    (:then_0
      (Default|RemoveCurrency (Variables|Runtime|GetGameMode) (Math|Conversions|ToFloat(Integer) (Variables|/Game/PowerGame/Currency/PDA_Purchase.PDA_Purchase_C|GetCost (Variables|Setup|GetPurchase)))))
    (:then_1
      (if (!= _levelunlock "")
        (Default|UnlockZone (Variables|Runtime|GetGameMode) _levelunlock)
        (Development|PrintString (Utilities|String|ToString(Name) _levelunlock))
        (else
          (Utilities|FlowControl|Sequence
            (:then_0
              (for (_array_element _array_index) (Variables|Runtime|GetTargetClasses)
                (bind _returnvalue (Game|SpawnActorfromClass _array_element (Utilities|Array|Get(acopy) (Variables|Runtime|GetTargetTransforms) _array_index) "Undefined" "MultiplyWithRoot" 0 0))
                (Utilities|Array|Add (LocalVariables|GetPurchasedActors) _returnvalue)))
            (:then_1
              (for _array_element_2 (Variables|Setup|GetActorAdditions)
                (Utilities|IsValid _array_element_2
                  (:Is%20Valid
                    (bind _returnvalue_2 (Game|SpawnActorfromClass (.Value (Utilities|Map|Find (Variables|Setup|GetActorUpgrades) (Utilities|GetClass _array_element_2))) (Transformation|GetActorTransform _array_element_2) "AlwaysSpawn" "MultiplyWithRoot" 0 0))
                    (Utilities|Array|Add (LocalVariables|GetPurchasedActors) _returnvalue_2)
                    (Actor|DestroyActor _array_element_2)))))))))
    (:then_2
      (Default|CallOnPurchased self (LocalVariables|GetPurchasedActors))
      (return))))