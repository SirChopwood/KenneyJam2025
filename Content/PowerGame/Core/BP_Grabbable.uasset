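; Grabbable physics actor that a player can pick up through Interact and release through Drop.
; Interact acts only when the player holds nothing, turning off the actor's collision and root physics before passing itself to the player's Grab.
; Drop detaches the actor with relative transforms kept, then restores collision and physics simulation.
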(event Custom|Drop
  (Transformation|DetachFromActor "KeepRelative" "KeepRelative" "KeepRelative")
  (Collision|SetActorEnableCollision true)
  (Physics|SetSimulatePhysics (Variables|Default|GetRoot) true))

(event EventBeginPlay)

(event Collision|EventActorBeginOverlap
  (params (OtherActor :type Actor%20Object%20Reference)))

(event EventTick
  (params (DeltaSeconds :type Float%20%28single-precision%29)))

(event EventInteract
  (params (Player :type BP%20Power%20Game%20Player%20Object%20Reference))
  (if (not (.ReturnValue (Default|GetGrabbedObject Player)))
    (Collision|SetActorEnableCollision false)
    (Physics|SetSimulatePhysics (Variables|Default|GetRoot) false)
    (Default|Grab Player self)))

(fn ConstructionScript)