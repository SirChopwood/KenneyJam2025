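; Player character for PowerGame that can interact with, pick up and drop objects.
; The interact input runs a vertical sphere trace just ahead, ignoring the held object, and passes hits to the actor's BP_grabbableComponent.
; With no hit, it drops and clears any held object.
; The Grab event stores the object, snaps it to the Hands component keeping world rotation, and plays a holding montage.
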(event Custom|Grab
  (params (ObjectToGrab :type Actor%20Object%20Reference))
  (bind _output_get (Variables|Default|SetGrabbedObject ObjectToGrab))
  (Transformation|AttachComponentToComponent _output_get (Variables|Default|GetHands) "" "SnapToTarget" "KeepWorld" "KeepRelative" true)
  (Animation|Montage|PlayMontage (Variables|Character|GetMesh) "/Game/PowerGame/Assets/Characters/kenney_mini-characters/character-female-d/SkeletalMeshes/holding-both_Montage.holding-both_Montage"))

(event Input|EnhancedActionEvents|EnhancedInputActionIA_Interact
  (params (ActionValue :type Boolean) (ElapsedSeconds :type Float%20%28double-precision%29) (TriggeredSeconds :type Float%20%28double-precision%29) (InputAction :type Input%20Action%20Object%20Reference :default "/Game/Input/Actions/IA_Interact.IA_Interact"))
  (bind _returnvalue (Transformation|GetActorForwardVector))
  (bind _returnvalue_2 (Transformation|GetActorLocation))
  (bind (_returnvalue_3 _grabbedobject1) (CallFunction|GetGrabbedObject))
  (bind _returnvalue_4 (* _returnvalue 5e+01))
  (bind _returnvalue_5 (+ _returnvalue_4 _returnvalue_2))
  (bind (_x _y _z) (Math|Vector|BreakVector _returnvalue_5))
  (bind (_outhit _returnvalue_6) (Collision|SphereTraceByChannel (Math|Vector|MakeVector _x _y (- _z 1e+02)) (Math|Vector|MakeVector _x _y (+ _z 1e+01)) 6e+01 "TraceTypeQuery3" false (Utilities|Array|MakeArray (Variables|Default|GetGrabbedObject)) "None"))
  (if _returnvalue_6
    (Class|BPIInteractable|Interact(Message) (Actor|GetComponentbyClass (.HitActor (Collision|BreakHitResult _outhit)) "/Game/PowerGame/Core/BP_grabbableComponent.BP_grabbableComponent_C") self)
    (elif _returnvalue_3
      (Default|Drop (Actor|GetComponentbyClass _grabbedobject1 "/Game/PowerGame/Core/BP_grabbableComponent.BP_grabbableComponent_C"))
      (Variables|Default|SetGrabbedObject 0))))

(fn ConstructionScript)

(fn GetGrabbedObject
  (bind _grabbedobject (Variables|Default|GetGrabbedObject))
  (return (Utilities|IsValid _grabbedobject) _grabbedobject))