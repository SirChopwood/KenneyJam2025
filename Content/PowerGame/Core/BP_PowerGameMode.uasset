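; BP_PowerGameMode is the game mode that tracks a player currency total and unlocks zones.
; UnlockZone loads the named streaming level as visible, blocking on load, then prints the level name on screen.
; AddCurrency and RemoveCurrency adjust the Currency variable directly, with no bounds checks.
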(event Custom|UnlockZone
  (params (LevelName :type Name))
  (Game|LoadStreamLevel(byName) LevelName true true)
  (Development|PrintString (Utilities|String|ToString(Name) LevelName) true true "(R=1.000000,G=0.007076,B=0.000000,A=1.000000)"))

(fn ConstructionScript)

(fn AddCurrency
  (params (Amount :type Float%20%28double-precision%29))
  (Variables|Default|SetCurrency (+ Amount (Variables|Default|GetCurrency))))

(fn RemoveCurrency
  (params (Amount :type Float%20%28double-precision%29))
  (Variables|Default|SetCurrency (- (Variables|Default|GetCurrency) Amount)))