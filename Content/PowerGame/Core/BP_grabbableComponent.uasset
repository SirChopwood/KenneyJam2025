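; Actor component that makes its owning actor a physics object the player can pick up and drop.
; Interact does nothing if the player already holds an object; otherwise it disables the owner's collision and root physics simulation, then passes the owner to the player's Grab.
; Drop detaches the owner with relative transform rules, then re-enables collision and physics on its root primitive.
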(event Custom|Drop
  (bind _returnvalue (Components|GetOwner))
  (Transformation|DetachFromActor (Components|GetOwner) "KeepRelative" "KeepRelative" "KeepRelative")
  (Collision|SetActorEnableCollision _returnvalue true)
  (bind _asprimitive_component (Utilities|Casting|CastToPrimitiveComponent (Variables|/Script/Engine.Actor|GetRootComponent _returnvalue)))
  (Physics|SetSimulatePhysics _asprimitive_component true))

(event EventBeginPlay)

(event EventTick
  (params (DeltaSeconds :type Float%20%28single-precision%29)))

(event EventInteract
  (params (Player :type BP%20Power%20Game%20Player%20Object%20Reference))
  (bind _returnvalue (Components|GetOwner))
  (if (not (.ReturnValue (Default|GetGrabbedObject Player)))
    (Collision|SetActorEnableCollision _returnvalue false)
    (bind _asprimitive_component (Utilities|Casting|CastToPrimitiveComponent (Variables|/Script/Engine.Actor|GetRootComponent _returnvalue)))
    (Physics|SetSimulatePhysics _asprimitive_component false)
    (Default|Grab Player (Components|GetOwner))))