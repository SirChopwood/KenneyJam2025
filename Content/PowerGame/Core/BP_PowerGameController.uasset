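; BP_PowerGameController is the player controller for the Power Game, setting up the HUD and cursor-driven input.
; On BeginPlay it casts the game mode to BP_PowerGameMode, passes it to a new WBP_HUD, shows that widget and enables game-and-UI input with a visible mouse cursor.
; Two debug keys add a small or large amount of currency through the game mode.
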(event EventBeginPlay
  (bind _asbp_power_game_mode (Utilities|Casting|CastToBP_PowerGameMode (Game|GetGameMode)))
  (bind _output_get (Variables|Default|SetGameMode _asbp_power_game_mode))
  (bind _returnvalue (UserInterface|CreateWidget "/Game/PowerGame/UI/WBP_HUD.WBP_HUD_C"))
  (Variables|/Game/PowerGame/UI/WBP_HUD.WBP_HUD_C|SetGameMode _returnvalue _output_get)
  (bind _output_get_2 (Variables|Default|SetHUD _returnvalue))
  (UserInterface|Viewport|AddtoViewport _output_get_2 0)
  (Input|SetInputModeGameandUI self _output_get_2 "DoNotLock" false false)
  (Variables|Default|SetbShowMouseCursor true))

(event Input|KeyboardEvents|DebugKey1
  (params (Key :type Key%20Structure :default "None") (ActionValue :type Input%20Action%20Value%20Structure))
  (:Pressed
    (Default|AddCurrency (Variables|Default|GetGameMode) 5e+01)))

(event Input|KeyboardEvents|DebugKey2
  (params (Key :type Key%20Structure :default "None") (ActionValue :type Input%20Action%20Value%20Structure))
  (:Pressed
    (Default|AddCurrency (Variables|Default|GetGameMode) 5e+02)))

(fn ConstructionScript)