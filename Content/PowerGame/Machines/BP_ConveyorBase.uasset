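; Base conveyor belt machine that pushes overlapping item actors along its belt direction.
; One tick after BeginPlay, yaw-rotated sphere traces find neighboring conveyors and destroy the matching right, back or left edge components.
; Each tick, items in PushField get a physics force along the combined actor and Direction rotation, reduced by their velocity along that axis relative to a speed term.
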(event EventBeginPlay
  (bind _returnvalue (Transformation|GetActorLocation))
  (Utilities|FlowControl|DelayUntilNextTick)
  (for (_array_element _array_index) (Variables|Default|GetCardinalDirections)
    (bind _outhits (Collision|MultiSphereTraceByChannel _returnvalue (+ _returnvalue (* (Math|Vector|RotateVectorAroundAxis _array_element (.yaw (Transformation|GetActorRotation)) "0.000000,0.000000,1.000000") (Variables|Default|GetCheckDistance)) "0.000000,0.000000,30.000000") 1e+01 "TraceTypeQuery1" false 0 "ForDuration"))
    (for _array_element_2 _outhits
      (Utilities|IsValid (.hitactor _array_element_2)
        (:Is%20Valid
          (if (Class|GameplayStatics|ObjectIsA (.hitactor _array_element_2) "BP_ConveyorBase_C")
            (for _array_element_3 (Components|GetChildrenComponents (Utilities|Select :Index _array_index :Option%200 (Variables|Default|GetRightEdge) :Option%201 (Variables|Default|GetBackEdge) :Option%202 (Variables|Default|GetLeftEdge)) true)
              (Utilities|IsValid _array_element_3
                (:Is%20Valid
                  (Components|DestroyComponent (Components|GetChildrenComponents (Utilities|Select :Index _array_index :Option%200 (Variables|Default|GetRightEdge) :Option%201 (Variables|Default|GetBackEdge) :Option%202 (Variables|Default|GetLeftEdge)) true)))))
            (Utilities|IsValid (Utilities|Select :Index _array_index :Option%200 (Variables|Default|GetRightEdge) :Option%201 (Variables|Default|GetBackEdge) :Option%202 (Variables|Default|GetLeftEdge))
              (:Is%20Valid
                (Components|DestroyComponent (Utilities|Select :Index _array_index :Option%200 (Variables|Default|GetRightEdge) :Option%201 (Variables|Default|GetBackEdge) :Option%202 (Variables|Default|GetLeftEdge)))))))))))

(event EventTick
  (params (DeltaSeconds :type Float%20%28single-precision%29))
  (bind _returnvalue (Transformation|GetActorRotation))
  (bind _force (Variables|Default|GetForce))
  (bind _direction (Variables|Default|GetDirection))
  (bind _maxspeedmultiplier (Variables|Default|GetMaxSpeedMultiplier))
  (bind _returnvalue_2 (Math|Rotator|CombineRotators _returnvalue _direction))
  (bind _returnvalue_3 (* _force _maxspeedmultiplier))
  (bind _returnvalue_4 (Math|Rotator|GetRotationXVector _returnvalue_2))
  (for _array_element (Collision|GetOverlappingActors (Variables|Default|GetPushField) "/Game/PowerGame/Machines/BP_ItemBase.BP_ItemBase_C" :!class /Script/Engine.PrimitiveComponent)
    (bind _asbp_item_base (Utilities|Casting|CastToBP_ItemBase _array_element))
    (Physics|AddForce (Variables|/Game/PowerGame/Machines/BP_ItemBase.BP_ItemBase_C|GetStaticMesh _asbp_item_base) (* (- (* (* _force (Variables|Default|GetForceMultiplier) DeltaSeconds) _returnvalue_3) (/ (Math|Vector|VectorLength (* _returnvalue_4 (Transformation|GetVelocity _array_element))) _returnvalue_3)) _returnvalue_4) "None" false)))

(fn ConstructionScript)