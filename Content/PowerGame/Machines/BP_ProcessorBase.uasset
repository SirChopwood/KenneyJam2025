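; Base processor machine that converts physics items into other items according to its Recipe.
; When an actor overlaps the ConversionPoint and its class exactly matches the Recipe's input item, SwapItems destroys it and spawns the output item at SpawnPoint.
; The new item's mesh receives the old item's velocity, so motion carries through the conversion.
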(event OnComponentBeginOverlap(ConversionPoint)
  (params (OverlappedComponent :type Primitive%20Component%20Object%20Reference) (OtherActor :type Actor%20Object%20Reference) (OtherComp :type Primitive%20Component%20Object%20Reference) (OtherBodyIndex :type Integer) (bFromSweep :type Boolean) (SweepResult :type Hit%20Result%20Structure%20%28by%20ref%29))
  (Utilities|IsValid (Variables|Default|GetRecipe)
    (:Is%20Valid
      (if (== (Utilities|GetClass OtherActor) (Variables|/Game/PowerGame/Machines/PDA_ProcessorRecipe.PDA_ProcessorRecipe_C|GetInput%20Item (Variables|Default|GetRecipe)))
        (bind _asbp_item_base (Utilities|Casting|CastToBP_ItemBase OtherActor))
        (CallFunction|SwapItems _asbp_item_base)))))

(event EventBeginPlay)

(event Collision|EventActorBeginOverlap
  (params (OtherActor :type Actor%20Object%20Reference)))

(event EventTick
  (params (DeltaSeconds :type Float%20%28single-precision%29)))

(fn ConstructionScript)

(fn SwapItems
  (params (OldItem :type BP%20Item%20Base%20Object%20Reference))
  (bind _spawnpoint (Variables|Default|GetSpawnPoint))
  (bind _returnvalue (Transformation|GetWorldTransform _spawnpoint))
  (LocalVariables|SetOldVelocity (Transformation|GetVelocity OldItem))
  (Actor|DestroyActor OldItem)
  (bind _returnvalue_2 (Game|SpawnActorfromClass (Variables|/Game/PowerGame/Machines/PDA_ProcessorRecipe.PDA_ProcessorRecipe_C|GetOutput%20Item (Variables|Default|GetRecipe)) (Math|Transform|MakeTransform (.location _returnvalue) (.rotation _returnvalue) "1.000000,1.000000,1.000000") "Undefined" "MultiplyWithRoot" 0 0))
  (Physics|SetPhysicsLinearVelocity (Variables|/Game/PowerGame/Machines/BP_ItemBase.BP_ItemBase_C|GetStaticMesh _returnvalue_2) (LocalVariables|GetOldVelocity) false "None"))