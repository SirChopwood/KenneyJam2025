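; BP_SpawnerComponent is a component that repeatedly spawns actors of a configured class for its owning actor.
; On BeginPlay it starts a looping timer whose interval and first delay are the inverse of SpawnRate, making the rate spawns per second.
; Each tick of that timer spawns Target's actor class at the owner's location plus the SpawnPoint offset, unrotated, with the owner and SpawnPoint rotations combined.
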(event Custom|Spawn%20Item
  (bind _returnvalue (Components|GetOwner))
  (bind _spawnpoint (Variables|Default|GetSpawnPoint))
  (bind _returnvalue_2 (Transformation|GetActorTransform _returnvalue))
  (Game|SpawnActorfromClass (Variables|/Game/PowerGame/Machines/PDA_SpawnerTarget.PDA_SpawnerTarget_C|GetActor (Variables|Default|GetTarget)) (Math|Transform|MakeTransform (+ (.location _returnvalue_2) (.location _spawnpoint)) (Math|Rotator|CombineRotators (.rotation _returnvalue_2) (.rotation _spawnpoint)) "1.000000,1.000000,1.000000") "Undefined" "MultiplyWithRoot" 0 0))

(event EventBeginPlay
  (bind _spawnrate (Variables|Default|GetSpawnRate))
  (bind _returnvalue (/ 1.0 _spawnrate))
  (Utilities|Time|SetTimerbyEvent (delegate Custom|Spawn%20Item) _returnvalue true false _returnvalue))