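; BP_SpawnerBase is a machine Blueprint, named as a base spawner, that repeatedly spawns a configurable actor class.
; On BeginPlay it starts a looping timer whose interval is the inverse of its Rate variable, so Rate acts as spawns per second.
; Each tick of the timer spawns the actor at the spawner's location plus an unrotated SpawnPoint offset, with SpawnRotation combined into the spawner's rotation.
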(event Custom|Spawn%20Item
  (bind _returnvalue (Transformation|GetActorTransform))
  (Game|SpawnActorfromClass (Variables|/Game/PowerGame/Machines/PDA_SpawnerTarget.PDA_SpawnerTarget_C|GetActor (Variables|Default|GetTarget)) (Math|Transform|MakeTransform (+ (.location _returnvalue) (Variables|Default|GetSpawnPoint)) (Math|Rotator|CombineRotators (.rotation _returnvalue) (Variables|Default|GetSpawnRotation)) "1.000000,1.000000,1.000000") "Undefined" "MultiplyWithRoot" 0 0))

(event EventBeginPlay
  (Utilities|Time|SetTimerbyEvent (delegate Custom|Spawn%20Item) (/ 1.0 (Variables|/Game/PowerGame/Machines/PDA_SpawnerTarget.PDA_SpawnerTarget_C|GetRate (Variables|Default|GetTarget))) true))

(fn ConstructionScript)