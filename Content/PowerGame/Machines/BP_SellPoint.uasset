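; BP_SellPoint is a machine that consumes items entering its SellZone and turns them into energy.
; On overlap, it passes the item's energy value and time to its electricity component's EnergyCreate, then destroys the item.
; It then calls EnergyTransfer with a multiplier times value over time, or times value alone when time is zero.
; The game mode is cached, but the AddCurrency call is unconnected, so no currency is awarded.
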(event OnComponentBeginOverlap(SellZone)
  (params (OverlappedComponent :type Primitive%20Component%20Object%20Reference) (OtherActor :type Actor%20Object%20Reference) (OtherComp :type Primitive%20Component%20Object%20Reference) (OtherBodyIndex :type Integer) (bFromSweep :type Boolean) (SweepResult :type Hit%20Result%20Structure%20%28by%20ref%29))
  (bind _bp_electricitycomponent (Variables|Default|GetBP_ElectricityComponent))
  (bind _asbp_item_base (Utilities|Casting|CastToBP_ItemBase OtherActor))
  (Default|EnergyCreate _bp_electricitycomponent (Variables|/Game/PowerGame/Machines/BP_ItemBase.BP_ItemBase_C|GetEnergyValue _asbp_item_base) (Variables|/Game/PowerGame/Machines/BP_ItemBase.BP_ItemBase_C|GetTime _asbp_item_base))
  (if (!= (Variables|/Game/PowerGame/Machines/BP_ItemBase.BP_ItemBase_C|GetTime _asbp_item_base) 0.0)
    (Actor|DestroyActor _asbp_item_base)
    (Default|EnergyTransfer _bp_electricitycomponent (* (Variables|Default|GetEnergyTransferAmountMulti) (/ (Variables|/Game/PowerGame/Machines/BP_ItemBase.BP_ItemBase_C|GetEnergyValue _asbp_item_base) (Variables|/Game/PowerGame/Machines/BP_ItemBase.BP_ItemBase_C|GetTime _asbp_item_base))))
    (else
      (Actor|DestroyActor _asbp_item_base)
      (Default|EnergyTransfer _bp_electricitycomponent (* (Variables|Default|GetEnergyTransferAmountMulti) (Variables|/Game/PowerGame/Machines/BP_ItemBase.BP_ItemBase_C|GetEnergyValue _asbp_item_base))))))

(event EventBeginPlay
  (bind _asbp_power_game_mode (Utilities|Casting|CastToBP_PowerGameMode (Game|GetGameMode)))
  (Variables|Default|SetAs%20BP%20Power%20Game%20Mode _asbp_power_game_mode))

(fn ConstructionScript)