(event Custom|EnergyDestroy
  (params (EnergyAmount :type Float%20%28double-precision%29) (Time :type Float%20%28double-precision%29))
  (if (> Time 0.0)
    (Variables|EnergyGain|SetEnergyTickAmount (/ EnergyAmount Time))
    (bind _returnvalue (Utilities|Time|SetTimerbyEvent (delegate Custom|EnergyTickSubtract) 0.1 true))
    (Variables|Default|SetTimer _returnvalue)
    (Utilities|Time|SetTimerbyEvent (delegate Custom|StopTimer1) Time)
    (Variables|Default|SetEnergy (Variables|EnergyGain|GetEnergyOverTime))
    (else
      (Variables|Default|SetEnergy (- (Variables|Default|GetEnergy) EnergyAmount)))))

(event Custom|EnergyTickSubtract
  (Variables|EnergyLoss|SetEnergyLossOverTime (- (Variables|EnergyLoss|GetEnergyLossOverTime) (Variables|EnergyLoss|GetEnergyLossTickAmount))))

(event Custom|StopTimer1
  (Utilities|Time|ClearandInvalidateTimerbyHandle (Variables|Default|GetTimer)))

(event Custom|EnergyTickAdd
  (Variables|EnergyGain|SetEnergyOverTime (+ (Variables|EnergyGain|GetEnergyOverTime) (Variables|EnergyGain|GetEnergyTickAmount))))

(event Custom|EnergyTransfer
  (params (EnergyAmount :type Float%20%28double-precision%29) (ItemType :type BP%20Item%20Base%20Object%20Reference))
  (bind _wire (Variables|Default|GetWire))
  (bind _energyflowrate (Variables|Default|GetEnergyFlowRate))
  (if (<= EnergyAmount _energyflowrate)
    (Variables|/Game/PowerGame/Electricity/BP_Wire.BP_Wire_C|SetEnergy _wire EnergyAmount)
    (else
      (Variables|/Game/PowerGame/Electricity/BP_Wire.BP_Wire_C|SetEnergy _wire (- EnergyAmount (- EnergyAmount _energyflowrate)))))
  (Variables|/Game/PowerGame/Electricity/BP_Wire.BP_Wire_C|SetSource _wire (Utilities|GetClassDisplayName (Utilities|GetClass ItemType))))

(event Custom|EnergyRecive
  (bind _wire (Variables|Default|GetWire))
  (bind _energyflowrate (Variables|Default|GetEnergyFlowRate))
  (bind _wire_2 (Variables|Default|GetWire))
  (bind _maxcapacity (Variables|Default|GetMaxCapacity))
  (bind _currentenergystored (Variables|Default|GetCurrentEnergyStored))
  (bind _returnvalue (- _maxcapacity _currentenergystored))
  (Variables|Default|SetRecivedSource (Variables|/Game/PowerGame/Electricity/BP_Wire.BP_Wire_C|GetSource _wire_2))
  (if (<= (Variables|/Game/PowerGame/Electricity/BP_Wire.BP_Wire_C|GetEnergy _wire_2) _energyflowrate)
    (if (<= (Variables|/Game/PowerGame/Electricity/BP_Wire.BP_Wire_C|GetEnergy _wire_2) _returnvalue)
      (Variables|Default|SetEnergy (Variables|/Game/PowerGame/Electricity/BP_Wire.BP_Wire_C|GetEnergy _wire_2))
      (Variables|/Game/PowerGame/Electricity/BP_Wire.BP_Wire_C|SetEnergy _wire 0.0)
      (else
        (Variables|Default|SetEnergy (- (Variables|/Game/PowerGame/Electricity/BP_Wire.BP_Wire_C|GetEnergy _wire_2) (- (Variables|/Game/PowerGame/Electricity/BP_Wire.BP_Wire_C|GetEnergy _wire_2) _returnvalue)))
        (Variables|/Game/PowerGame/Electricity/BP_Wire.BP_Wire_C|SetEnergy _wire 0.0)))
    (elif (<= (- (Variables|/Game/PowerGame/Electricity/BP_Wire.BP_Wire_C|GetEnergy _wire_2) (- (Variables|/Game/PowerGame/Electricity/BP_Wire.BP_Wire_C|GetEnergy _wire_2) _energyflowrate)) _returnvalue)
      (Variables|Default|SetEnergy (- (Variables|/Game/PowerGame/Electricity/BP_Wire.BP_Wire_C|GetEnergy _wire_2) (- (Variables|/Game/PowerGame/Electricity/BP_Wire.BP_Wire_C|GetEnergy _wire_2) _energyflowrate)))
      (Variables|/Game/PowerGame/Electricity/BP_Wire.BP_Wire_C|SetEnergy _wire 0.0)
      (else
        (Variables|Default|SetEnergy (- (- (Variables|/Game/PowerGame/Electricity/BP_Wire.BP_Wire_C|GetEnergy _wire_2) (- (Variables|/Game/PowerGame/Electricity/BP_Wire.BP_Wire_C|GetEnergy _wire_2) _energyflowrate)) (- (- (Variables|/Game/PowerGame/Electricity/BP_Wire.BP_Wire_C|GetEnergy _wire_2) (- (Variables|/Game/PowerGame/Electricity/BP_Wire.BP_Wire_C|GetEnergy _wire_2) _energyflowrate)) _returnvalue)))
        (Variables|/Game/PowerGame/Electricity/BP_Wire.BP_Wire_C|SetEnergy _wire 0.0)))))

(event Custom|StopTimer2
  (Utilities|Time|ClearandInvalidateTimerbyHandle (Variables|Default|GetTimer)))

(event Custom|EnergyCreate
  (params (EnergyAmount :type Float%20%28double-precision%29) (Time :type Float%20%28double-precision%29))
  (if (> Time 0.0)
    (Variables|EnergyGain|SetEnergyTickAmount (/ EnergyAmount Time))
    (bind _returnvalue (Utilities|Time|SetTimerbyEvent (delegate Custom|EnergyTickAdd) 0.1 true))
    (Variables|Default|SetTimer _returnvalue)
    (Utilities|Time|SetTimerbyEvent (delegate Custom|StopTimer2) Time)
    (Variables|Default|SetEnergy (Variables|EnergyGain|GetEnergyOverTime))
    (else
      (Variables|Default|SetEnergy EnergyAmount))))

(event EventBeginPlay
  (bind _returnvalue (Actor|GetActorOfClass "/Game/PowerGame/Electricity/BP_Wire.BP_Wire_C"))
  (bind _output_get (Variables|Default|SetWire _returnvalue))
  (Variables|/Game/PowerGame/Electricity/BP_Wire.BP_Wire_C|SetEnergy _output_get 1.0))

(event EventTick
  (params (DeltaSeconds :type Float%20%28single-precision%29)))